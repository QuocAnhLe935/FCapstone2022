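; VR teleport visualizer that draws the player's play area bounds through a Niagara system to preview the area after a teleport.
; On BeginPlay it passes the stage play area size to the Niagara system.
; Each Tick it offsets the system by the negated horizontal HMD position in pawn space and applies the pawn's rotation, so the bounds reflect where the player stands within the new area.
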(event EventBeginPlay
  (bind _returnvalue (Class|HeadMountedDisplayFunctionLibrary|GetPlayAreaBounds "Stage"))
  (Niagara|SetNiagaraVariable(Vector3) (Variables|Default|GetNS_PlayAreaBounds) "User PlayAreaBounds" (Math|Vector|MakeVector (.x _returnvalue) (.y _returnvalue) 0.0)))

(event EventTick
  (params (DeltaSeconds :type Float%20%28single-precision%29))
  (bind _returnvalue (Game|Player|GetPlayerPawn 0))
  (bind _returnvalue_2 (Game|GetPlayerCameraManager 0))
  (bind _returnvalue_3 (Transformation|GetActorTransform _returnvalue))
  (bind _returnvalue_4 (Camera|GetCameraLocation _returnvalue_2))
  (bind _returnvalue_5 (Math|Transform|InverseTransformLocation _returnvalue_3 _returnvalue_4))
  (bind _returnvalue_6 (Math|Vector|NegateVector _returnvalue_5))
  ;[1 1 1] Move the play area bounds of the Niagara system relative to the players HMD location in the new play area
  (Transformation|SetRelativeLocationAndRotation (Variables|Default|GetNS_PlayAreaBounds) (Math|Vector|MakeVector (.x _returnvalue_6) (.y _returnvalue_6) 0.0) (Transformation|GetActorRotation (Game|Player|GetPlayerPawn 0)) false false))

(fn ConstructionScript)