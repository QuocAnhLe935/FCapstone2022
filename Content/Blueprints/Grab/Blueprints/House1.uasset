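; House1 is a Blueprint with a static mesh that stays upright and locked to 90-degree world rotations.
; Every Tick, it reads the mesh's world yaw, rounds it to the nearest quarter turn with a math expression, and writes it back with zero pitch and roll.
; BeginPlay, overlap and the construction script do nothing.
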(event EventBeginPlay)

(event Collision|EventActorBeginOverlap
  (params (OtherActor :type Actor%20Object%20Reference)))

(event EventTick
  (params (DeltaSeconds :type Float%20%28single-precision%29))
  ;[1 1 1] Keep Object at 90 degree Rotations
  (Transformation|SetWorldRotation (Variables|Default|GetStaticMesh) (Math|Rotator|MakeRotator 0.0 0.0 (Math|Conversions|ToFloat(Integer) (|((round((direction/90)))*90) (.yaw (Transformation|GetWorldRotation (Variables|Default|GetStaticMesh)))))) false false))

(fn ConstructionScript)