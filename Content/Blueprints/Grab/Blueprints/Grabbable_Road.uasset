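; Grabbable road piece that keeps its static mesh aligned to 90-degree yaw steps.
; Every Tick, a chain of range checks on the mesh's world yaw snaps it to the nearest quarter turn, leaving pitch and roll unchanged.
; The checks assume a 0–360 yaw, so any negative yaw falls into the first branch and snaps to zero.
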(event EventBeginPlay)

(event EventTick
  (params (DeltaSeconds :type Float%20%28single-precision%29))
  (bind _staticmesh (Variables|Default|GetStaticMesh))
  (bind _staticmesh_2 (Variables|Default|GetStaticMesh))
  (bind _staticmesh_3 (Variables|Default|GetStaticMesh))
  (bind _staticmesh_4 (Variables|Default|GetStaticMesh))
  (bind _staticmesh_5 (Variables|Default|GetStaticMesh))
  (bind _returnvalue (Transformation|GetWorldRotation _staticmesh_3))
  (bind _returnvalue_2 (Transformation|GetWorldRotation _staticmesh_4))
  (bind _returnvalue_3 (Transformation|GetWorldRotation _staticmesh_5))
  (bind _returnvalue_4 (Transformation|GetWorldRotation _staticmesh))
  (bind _returnvalue_5 (Transformation|GetWorldRotation _staticmesh_2))
  ;[1 1 1] If Rotation is < 45 or > 315 set rotation to 0
  (if (or (< (.yaw _returnvalue_5) 45.0) (> (.yaw _returnvalue_5) 315.0))
    (Transformation|SetWorldRotation _staticmesh_3 (Math|Rotator|MakeRotator (.roll _returnvalue) (.pitch _returnvalue) 0.0) false false)
    (else
      ;[1 1 1] If Rotation is < 135 or > 45 set rotation to 90
      (if (Math|Float|InRange(Float) (.yaw (Transformation|GetWorldRotation (Variables|Default|GetStaticMesh))) 45.0 135.0)
        (Transformation|SetWorldRotation _staticmesh_4 (Math|Rotator|MakeRotator (.roll _returnvalue_2) (.pitch _returnvalue_2) 9e+01) false false)
        (else
          ;[1 1 1] If Rotation is < 225 or > 135 set rotation to 0
          (if (Math|Float|InRange(Float) (.yaw (Transformation|GetWorldRotation (Variables|Default|GetStaticMesh))) 135.0 225.0)
            (Transformation|SetWorldRotation _staticmesh_5 (Math|Rotator|MakeRotator (.roll _returnvalue_3) (.pitch _returnvalue_3) 1.8e+02) false false)
            (else
              ;[1 1 1] If Rotation is < 225 or > 135 set rotation to 0
              (if (Math|Float|InRange(Float) (.yaw (Transformation|GetWorldRotation (Variables|Default|GetStaticMesh))) 225.0 315.0)
                (Transformation|SetWorldRotation _staticmesh (Math|Rotator|MakeRotator (.roll _returnvalue_4) (.pitch _returnvalue_4) 2.7e+02) false false)))))))))

(event Collision|EventActorBeginOverlap
  (params (OtherActor :type Actor%20Object%20Reference)))

(fn ConstructionScript)