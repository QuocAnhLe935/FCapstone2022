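; BP_Ghost_Building is a ghost building Blueprint in the Grab system that shows or hides a supplied display mesh.
; OnCreate stores the mesh and assigns it to GhostStaticMesh, ignoring further calls while IsActive is set.
; OnDestroy clears the mesh and resets the flag without destroying the actor, so the same ghost can be reused.
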(event Custom|OnCreate
  (params (DisplayMesh :type Static%20Mesh%20Object%20Reference))
  (if (not (Variables|Default|GetIsActive))
    (Variables|Default|SetDisplayMesh DisplayMesh)
    (Variables|Default|SetIsActive true)
    (Components|StaticMesh|SetStaticMesh (Variables|Default|GetGhostStaticMesh) (Variables|Default|GetDisplayMesh))))

(event Custom|OnDestroy
  (Variables|Default|SetDisplayMesh 0)
  (Variables|Default|SetIsActive false)
  (Components|StaticMesh|SetStaticMesh (Variables|Default|GetGhostStaticMesh) 0))

(fn ConstructionScript)